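; Test zombie that issues a move toward the player controller every tick and plays physics-based hit reactions; Die only prints a message.
; Hit maps the struck bone up toward spine_02 or a thigh, simulates physics below it and applies a force at the impact.
; A DoOnce-gated timeline drives the physics blend weight, then stops simulation.
; Physical animation settings are applied once at BeginPlay.
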(event `self.ReceiveTick`
  (params (DeltaSeconds :type "Float (single-precision)"))
  (`|AIMoveTo` (`self.CharacterMovement`) self (0.0 0.0 0.0) (`GameplayStatics.GetPlayerController` 0)))

(event `self.ReceiveBeginPlay`
  (`PhysicalAnimationComponent.SetSkeletalMeshComponent` (`self.PhysicalAnimation`) (`self.Mesh`))
  (`PhysicalAnimationComponent.ApplyPhysicalAnimationSettings` (`self.PhysicalAnimation`) (`self.PhysBone`) (make `PhysicalAnimationData` false 3000.0 80.0)))

(event `/Game/Blueprints/BPI_Die.Die`
  (params (HitLoc :type "Vector Structure") (HitDir :type "Vector Structure"))
  (`KismetSystemLibrary.PrintString` "Died"))

(event `/Game/Blueprints/BPI_Die.Hit`
  (params (HitLoc :type "Vector Structure") (HitDir :type "Vector Structure"))
  (bind _mesh (`self.Mesh`))
  (bind _mesh_2 (`self.Mesh`))
  (bind _physbone (`self.PhysBone`))
  (bind _mesh_3 (`self.Mesh`))
  (bind (_closestworldposition _normal _bonename) (`SkeletalMeshComponent.K2_GetClosestPointOnPhysicsAsset` _mesh (`self.Hit Loc`)))
  (set `self.Hit Loc` HitLoc)
  (bind _usethisbone (`self.FindParentBone` _bonename _mesh))
  (bind _output_get (set `self.PhysBone` _usethisbone))
  (`SkeletalMeshComponent.SetAllBodiesBelowSimulatePhysics` _mesh_2 _output_get true true)
  (`|ExecutionSequence`
    (:`then_0`
      (set `self.HitForce` (+ HitLoc (* (`KismetMathLibrary.Normal` HitDir) (`self.ForceMultiply`)))))
    (:`then_1`
      (`/Engine/EditorBlueprintResources/StandardMacros.DoOnce` false :!label _label
        (:`Completed`
          (`KismetSystemLibrary.Delay` 0.1)
          (bind (_direction _newtrack_0) (`Timeline|HitReact` :!via `PlayFromStart`)
            (:`Update`
              (`SkeletalMeshComponent.SetAllBodiesBelowPhysicsBlendWeight` _mesh_3 _physbone _newtrack_0 false true))
            (:`Finished`
              (`SkeletalMeshComponent.SetAllBodiesBelowSimulatePhysics` _mesh_3 _physbone false true)
              (goto _label :!via `Reset`))))))
    (:`then_2`
      (if (`SceneComponent.IsSimulatingPhysics` _mesh_2 _bonename)
        (`PrimitiveComponent.AddForceAtLocation` (`self.Mesh`) (`self.HitForce`) _closestworldposition _bonename)))))

(fn `FindParentBone`
  (params (HitBone :type Name) (NewParam :type "SkinnedMeshComponent Object Reference"))
  (returns (UseThisBone :type Name))
  (locals (bIsChild :type Boolean) (CurrentBone :type Name) (ParentBone :type Name))
  (bind _parentbone (`local.ParentBone`))
  (bind _output_get (set `local.CurrentBone` HitBone))
  (if (or (== _output_get "pelvis") (== (`SkinnedMeshComponent.GetParentBone` (`self.Mesh`) _output_get) "pelvis"))
    (set `local.ParentBone` "spine_02")
    (else
      (while (not (`local.bIsChild`))
        (bind _output_get_2 (set `local.ParentBone` (`SkinnedMeshComponent.GetParentBone` (`self.Mesh`) (`local.CurrentBone`))))
        (if (or (== _output_get_2 "spine_02") (== _output_get_2 "thigh_l") (== _output_get_2 "thigh_r"))
          (set `local.bIsChild` true)
          (elif (== _parentbone "none")
            (set `local.bIsChild` true)
            (else
              (bind _output_get_3 (set `local.CurrentBone` _parentbone))
              (`KismetSystemLibrary.PrintString` (`KismetStringLibrary.Conv_NameToString` _output_get_3))))))))
  (return (`local.ParentBone`)))

(fn `PlayHitReaction`)

(fn `UserConstructionScript`)