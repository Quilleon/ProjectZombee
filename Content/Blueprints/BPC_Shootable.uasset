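; BPC_Shootable is an actor component that gives its owner health and lets it react to being shot.
; On BeginPlay it caches the owner and adds an offset to health.
; HitReg stores hit location and direction, then applies fixed damage through TakeDamage, ignoring the bone.
; TakeDamage forwards a hit message to the owner and, at zero health, sends a one-time death message if the owner implements BPI_Die.
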(event `self.ReceiveBeginPlay`
  (bind _returnvalue (`self.GetOwner`))
  (`/Engine/EditorBlueprintResources/StandardMacros.IsValid` _returnvalue
    (:`Is Valid`
      (set `self.Owner` _returnvalue)
      (set `self.Health` (+ (`self.Health`) (`self.HealthOffset`))))))

(event `TakeDamage`
  (params (DmgAmount :type "Float (double-precision)") (HitLoc :type "Vector Structure") (HitDir :type "Vector Structure"))
  (message `/Game/Blueprints/BPI_Die.Hit` (`self.Owner`) (`self.Hit Location`) (`self.Hit Direction`))
  (set `self.Health` (- (`self.Health`) DmgAmount))
  (if (<= (`self.Health`) 0.0)
    (`self.Send Death`)))

(event `Send Death`
  (bind _owner (`self.Owner`))
  (`/Engine/EditorBlueprintResources/StandardMacros.DoOnce` false
    (:`Completed`
      (if (`KismetSystemLibrary.DoesImplementInterface` _owner "/Game/Blueprints/BPI_Die.BPI_Die_C")
        (message `/Game/Blueprints/BPI_Die.Die` _owner (`self.Hit Location`) (`self.Hit Direction`))))))

(fn `HitReg`
  (params (HitLocation :type "Vector Structure") (HitDirection :type "Vector Structure") (Bone :type Name))
  (bind _output_get (set `self.Hit Location` HitLocation))
  (bind _output_get_2 (set `self.Hit Direction` HitDirection))
  (`self.TakeDamage` 35.0 _output_get _output_get_2)
  (`KismetSystemLibrary.PrintString` "OOuch ")
  (return))