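; Manager actor for the zombie outbreak simulation: spawns a trace-checked grid of inhabitants and makes a random one patient zero.
; A Delay on Tick paces simulated days, each re-sorting inhabitants into Healthy, Bitten and Zombie arrays and advancing bitten ones toward turning.
; The population counts feed a zombie model, whose daily bite count is handed out to shuffled, unassigned zombies.
; When the model finishes, final counts go to BP_GameInstance and the score screen opens.
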(event `self.ReceiveBeginPlay`
  (bind _bitten_capacity (`self.Bitten_capacity`))
  (bind _spawndistance (`self.SpawnDistance`))
  (bind _returnvalue (`KismetMathLibrary.Sqrt` _bitten_capacity))
  ; Create zombie grid
  (for _index (range (+ (`KismetMathLibrary.FTrunc` _bitten_capacity) 1))
    (bind _returnvalue_2 (`KismetMathLibrary.Conv_IntToDouble` (+ _index (`self.Failed Zombiespawns`))))
    (bind _returnvalue_3 (+ (`self.K2_GetActorLocation` self) (`KismetMathLibrary.MakeVector` (`KismetMathLibrary.Conv_Int64ToDouble` (* (`KismetMathLibrary.Conv_DoubleToInt64` (/ _returnvalue_2 _returnvalue)) _spawndistance)) (* (mod _returnvalue_2 _returnvalue) _spawndistance))))
    (bind (_outhit _returnvalue_4) (`KismetSystemLibrary.CapsuleTraceSingle` _returnvalue_3 (+ _returnvalue_3 (`KismetMathLibrary.MakeVector` 0.0 0.0 100.0)) 50.0 100.0 "TraceTypeQuery1"))
    (if _returnvalue_4
      (`KismetSystemLibrary.PrintString` "failed to spawn" true true (struct :`R` 1.0 :`G` 0.059331 :`A` 1.0))
      (`/Engine/EditorBlueprintResources/StandardMacros.IncrementInt` (`self.Failed Zombiespawns`)
        (:`  `
          (`/Engine/EditorBlueprintResources/StandardMacros.DecrementInt` _index)))
      (else
        (bind _returnvalue_5 (`|SpawnActorFromClass` "/Game/Blueprints/BP_Innhabitant.BP_Innhabitant_C" (`KismetMathLibrary.Conv_VectorToTransform` _returnvalue_3) "Undefined" "MultiplyWithRoot" null null))
        (set `/Game/Blueprints/BP_Innhabitant.ZombieManager` self _returnvalue_5)
        (`KismetArrayLibrary.Array_Add` (`self.Innhabitants`) _returnvalue_5)
        (`KismetArrayLibrary.Array_Add` (`self.Healthy Innhabitants`) _returnvalue_5))))
  ; Assign Patient Zero
  (set `Innhabitant.currentState` "Zombie" (`KismetArrayLibrary.Array_Random` (`self.Healthy Innhabitants`))))

(event `self.ReceiveTick`
  (params (DeltaSeconds :type "Float (single-precision)"))
  (bind _tickduration (`self.TickDuration`))
  (bind _bitten_innhabitants (`self.Bitten Innhabitants`))
  (bind _bitestodistribute (`self.BitesToDistribute`))
  (bind _returnvalue (`KismetArrayLibrary.Array_Length` (`self.Healthy Innhabitants`)))
  (bind _returnvalue_2 (`KismetArrayLibrary.Array_Length` (`self.Zombie Innhabitants`)))
  (bind _returnvalue_3 (`KismetArrayLibrary.Array_Length` (`self.Bitten Innhabitants`)))
  (set `self.TimeUntilNextTick` (`KismetMathLibrary.FClamp` (- (`self.TimeUntilNextTick`) DeltaSeconds) 0.0 (`self.TickDuration`)))
  (`KismetSystemLibrary.Delay` _tickduration)
  (set `self.TimeUntilNextTick` _tickduration)
  ; Assign Enum Arrays
  (for _index (range 3)
    (switch `int` _index
      (:`0`
        (`self.Iterate over Array` "Healthy" (`self.Healthy Innhabitants`)))
      (:`1`
        (`self.Iterate over Array` "Bitten" _bitten_innhabitants :!label _label)
        (for _array_element _bitten_innhabitants
          (bind _infectiontakeover (`/Game/Blueprints/BP_Innhabitant.InfectionTakeover` _array_element))
          (if (< _infectiontakeover 15)
            (`/Engine/EditorBlueprintResources/StandardMacros.IncrementInt` _infectiontakeover)
            (else
              (set `Innhabitant.currentState` "Zombie" _array_element)
              (goto _label)))))
      (:`2`
        (`self.Iterate over Array` "Zombie" (`self.Zombie Innhabitants`)))))
  (`KismetSystemLibrary.PrintString` (`KismetStringLibrary.Concat_StrStr` "Healthy: " (`KismetStringLibrary.Conv_IntToString` _returnvalue) ", Bitten: " (`KismetStringLibrary.Conv_IntToString` _returnvalue_3) ", Zombies:" (`KismetStringLibrary.Conv_IntToString` _returnvalue_2)) true true (struct :`G` 0.66 :`B` 1.0 :`A` 1.0) 15.0)
  ; Run the model to figure out how many bites should occur today
  (`self.ZombieModel`)
  (bind (_bittentoday _finished) (`self.ZombieModelWithInputs` (`KismetMathLibrary.Conv_IntToDouble` _returnvalue) (`KismetMathLibrary.Conv_IntToDouble` _returnvalue_3) (`KismetMathLibrary.Conv_IntToDouble` _returnvalue_2)))
  (if _finished
    (`KismetSystemLibrary.PrintString` "Everyone is zombies" true true (struct :`G` 1.0 :`A` 1.0) 0.1)
    (`KismetSystemLibrary.Delay` 2.0)
    (bind _asbp_game_instance (cast `/Game/Blueprints/BP_GameInstance` (`GameplayStatics.GetGameInstance`)))
    (set `/Game/Blueprints/BP_GameInstance.Healthy` (`KismetArrayLibrary.Array_Length` (`self.Healthy Innhabitants`)) _asbp_game_instance)
    (set `/Game/Blueprints/BP_GameInstance.Bitten` (`KismetArrayLibrary.Array_Length` (`self.Bitten Innhabitants`)) _asbp_game_instance)
    (set `/Game/Blueprints/BP_GameInstance.Zombies` (`KismetArrayLibrary.Array_Length` (`self.Zombie Innhabitants`)) _asbp_game_instance)
    (`GameplayStatics.OpenLevel` "L_ScoreScreen")
    (else
      ; Destribute all bites and biters that should happen during the day
      (bind _output_get (set `self.BitesToDistribute` _bittentoday))
      (if (> _output_get 0)
        (bind _output_get_2 (set `self.TempArray` (`self.Zombie Innhabitants`)))
        (`KismetArrayLibrary.Array_Shuffle` _output_get_2)
        (for _array_element_2 _output_get_2
          (if (== (`/Game/Blueprints/BP_Innhabitant.Assigned Bites Today` _array_element_2) 0)
            (`/Game/Blueprints/BP_Innhabitant.AssignBitesToday` _array_element_2)
            (`/Engine/EditorBlueprintResources/StandardMacros.DecrementInt` (`self.BitesToDistribute`)
              (:`  `
                (if (not (> (`self.BitesToDistribute`) 0))
                  (break)))))))
      (if (not (== 0 _bitestodistribute))
        (`KismetSystemLibrary.PrintString` (`KismetStringLibrary.Concat_StrStr` "Missing " (`KismetStringLibrary.Conv_IntToString` _bitestodistribute) " bites to distribute") true true (struct :`R` 1.0 :`A` 1.0) 15.0)))))

(fn `Iterate over Array`
  (params (State :type "ZombieState Enum" :default "Healthy") (ActorArray :type "Array of /Game/Blueprints/BP_Innhabitant Object Reference"))
  (locals (TempCurrentState :type "ZombieState Enum"))
  (for _array_element ActorArray
    (if (`/Game/Blueprints/BP_Innhabitant.bDead` _array_element)
      (`KismetArrayLibrary.Array_RemoveItem` ActorArray _array_element :!label _label)
      (else
        (bind _currentstate (`Innhabitant.currentState` _array_element))
        (if (`|EnumInequality` _currentstate State)
          ; Add to correct array
          (switch `ZombieState` _currentstate
            (:`Healthy`
              (`KismetArrayLibrary.Array_Add` (`self.Healthy Innhabitants`) _array_element)
              (goto _label))
            (:`Bitten`
              (`KismetArrayLibrary.Array_Add` (`self.Bitten Innhabitants`) _array_element)
              (goto _label))
            (:`Zombie`
              (`KismetArrayLibrary.Array_Add` (`self.Zombie Innhabitants`) _array_element)
              (goto _label))))))))

(fn `UserConstructionScript`)