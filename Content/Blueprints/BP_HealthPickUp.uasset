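; Health pickup that spins, bobs on a timeline and sends OnPickUpMessage to overlapping actors implementing BPI_PickUp.
; A DoOnce gates pickup, and RespawnTimer hides the mesh and light for ten seconds before showing them and re-arming it.
; While the game instance's Caramell flag is set, timeline updates also brighten the light and pick its color from the MP_CaramellSettings Beat parameter.
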(event `self.ReceiveBeginPlay`
  (bind (_direction _newtrack_0) (`Timeline|UpAndDown` :!via `PlayFromStart`)
    (:`Update`
      (`SceneComponent.K2_AddWorldOffset` (`self.BoxRoot`) (`KismetMathLibrary.MakeVector` 0.0 0.0 (`KismetMathLibrary.MapRangeClamped` _newtrack_0 -1.0 1.0 -0.6 0.6)) false false)
      (`self.DiscoLightFunc`))))

(event `self.ReceiveTick`
  (params (DeltaSeconds :type "Float (single-precision)"))
  (`SceneComponent.K2_AddWorldRotation` (`self.BoxRoot`) (`KismetMathLibrary.MakeRotator` 0.0 0.0 (* DeltaSeconds 100.0)) false false))

(event `RespawnTimer`
  (bind _healthpackmesh (`self.HealthPackMesh`))
  (`SceneComponent.SetVisibility` _healthpackmesh false true)
  (`SceneComponent.SetVisibility` (`self.light`) false true)
  (`KismetSystemLibrary.Delay` 10.0)
  (`SceneComponent.SetVisibility` _healthpackmesh true true)
  (`SceneComponent.SetVisibility` (`self.light`) true true)
  (goto _label :!via `Reset`))

(event `self.Capsule.OnComponentBeginOverlap`
  (params (OverlappedComponent :type "PrimitiveComponent Object Reference") (OtherActor :type "Actor Object Reference") (OtherComp :type "PrimitiveComponent Object Reference") (OtherBodyIndex :type Integer) (bFromSweep :type Boolean) (SweepResult :type "HitResult Structure (by ref)"))
  (if (`KismetSystemLibrary.DoesImplementInterface` OtherActor "/Game/Blueprints/BPI_PickUp.BPI_PickUp_C")
    (`/Engine/EditorBlueprintResources/StandardMacros.DoOnce` false :!label _label
      (:`Completed`
        (message `/Game/Blueprints/BPI_PickUp.OnPickUp` OtherActor)
        (`self.RespawnTimer`)))))

(fn `DiscoLightFunc`
  (bind _light (`self.light`))
  (bind _light_2 (`self.light`))
  (`/Engine/EditorBlueprintResources/StandardMacros.IsValid` (`self.light`)
    (:`Is Valid`
      (bind _asbp_game_instance (cast `/Game/Blueprints/BP_GameInstance` (`GameplayStatics.GetGameInstance`)))
      (bind _returnvalue (`KismetMaterialLibrary.GetScalarParameterValue` "/Game/PostProcess/MP_CaramellSettings.MP_CaramellSettings" "Beat"))
      (if (`/Game/Blueprints/BP_GameInstance.Caramell?` _asbp_game_instance)
        (`LightComponent.SetIntensity` _light 20000.0)
        (`LightComponent.SetVolumetricScatteringIntensity` _light 1.0)
        (switch `int` (`KismetMathLibrary.FTrunc` _returnvalue)
          (:`Default`
            (`LightComponent.SetLightColor` _light_2 (struct :`R` 1.0 :`A` 1.0) true :!label _label))
          (:`0`
            (goto _label))
          (:`1`
            (`LightComponent.SetLightColor` _light_2 (struct :`R` 0.090871 :`G` 1.0 :`A` 1.0) true))
          (:`2`
            (`LightComponent.SetLightColor` _light_2 (struct :`R` 1.0 :`B` 0.9391 :`A` 1.0) true))
          (:`3`
            (`LightComponent.SetLightColor` _light_2 (struct :`G` 0.22852 :`B` 1.0 :`A` 1.0) true)))))))

(fn `UserConstructionScript`)